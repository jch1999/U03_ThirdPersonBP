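; Player character Blueprint with camera-relative movement, sprint, jump-based evade and a one-handed sword combat mode.
; BeginPlay spawns the sword and holsters it on a mesh socket; the OneHand input starts equip or unequip, locking movement and switching between strafe and orient-to-movement rotation.
; Separate events attach or detach the sword and finish state changes, gating the montage attack to the armed, idle state.
; A Regdoll function launches the physics-simulated mesh upward.
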(fn ConstructionScript)

(fn Regdoll
  (bind _mesh (Variables|Character|GetMesh))
  (Physics|SetSimulatePhysics _mesh true)
  (Collision|SetCollisionEnabled _mesh "PhysicsOnly")
  (Collision|SetCollisionEnabled (Variables|Collision|GetCapsuleComponent) "NoCollision")
  (Physics|AddForce (Variables|Character|GetMesh) "0, 0,10000000.000000" "None" false))

(event Input|ActionEvents|InputActionSprint
  (params (Key :type Key%20Structure :default "None"))
  (bind _charactermovement (Variables|Character|GetCharacterMovement))
  ;[1 1 1] Sprint
  (:Pressed
    (Variables|/Script/Engine.CharacterMovementComponent|SetMaxWalkSpeed _charactermovement 6e+02))
  (:Released
    (Variables|/Script/Engine.CharacterMovementComponent|SetMaxWalkSpeed _charactermovement 4e+02)))

(event Input|ActionEvents|InputActionEvade
  (params (Key :type Key%20Structure :default "None"))
  ;[1 1 1] Evade
  (:Pressed
    (Character|Jump))
  (:Released
    (Character|StopJumping)))

(event Input|AxisEvents|InputAxisMoveRight
  (params (AxisValue :type Float%20%28single-precision%29))
  ;[1 1 1] Movemnt
  (if (Variables|Default|GetbCanMove)
    (if (!= AxisValue 0.0)
      (Pawn|Input|AddMovementInput (Math|Vector|GetRightVector (Math|Rotator|MakeRotator 0.0 0.0 (.yaw (Pawn|GetControlRotation :!class /Script/Engine.Pawn)))) AxisValue false))))

(event Input|AxisEvents|InputAxisMoveForward
  (params (AxisValue :type Float%20%28single-precision%29))
  ;[1 1 1] Movemnt
  (if (Variables|Default|GetbCanMove)
    (if (!= AxisValue 0.0)
      (Pawn|Input|AddMovementInput (Math|Vector|GetForwardVector (Math|Rotator|MakeRotator 0.0 0.0 (.yaw (Pawn|GetControlRotation :!class /Script/Engine.Pawn)))) AxisValue false))))

(event Input|AxisEvents|InputAxisTurn
  (params (AxisValue :type Float%20%28single-precision%29))
  (Pawn|Input|AddControllerYawInput AxisValue))

(event Input|AxisEvents|InputAxisLookUp
  (params (AxisValue :type Float%20%28single-precision%29))
  (Pawn|Input|AddControllerPitchInput AxisValue))

(event Custom|EquippedOneHand
  ;[1 1 1] Equip
  (Variables|Default|SetStateType "NewEnumerator0")
  (Variables|Default|SetbCanMove true)
  (Variables|Default|SetCombatType "NewEnumerator1"))

(event Custom|EquipOneHand
  ;[1 1 1] Equip
  (Variables|Default|SetStateType "NewEnumerator1")
  (Variables|Default|SetbUseControllerRotationYaw true)
  (Variables|/Script/Engine.CharacterMovementComponent|SetbOrientRotationToMovement (Variables|Character|GetCharacterMovement) false)
  (Variables|Default|SetbCanMove false))

(event Custom|UnequipOneHand
  ;[1 1 1] Unequipped
  (Variables|Default|SetStateType "NewEnumerator2")
  (Variables|Default|SetbUseControllerRotationYaw false)
  (Variables|/Script/Engine.CharacterMovementComponent|SetbOrientRotationToMovement (Variables|Character|GetCharacterMovement) true)
  (Variables|Default|SetbCanMove false))

(event Custom|UnequippedOneHand
  ;[1 1 1] Unequipped
  (Variables|Default|SetStateType "NewEnumerator0")
  (Variables|Default|SetbCanMove true)
  (Variables|Default|SetCombatType "NewEnumerator0"))

(event Custom|AttachOneHand
  ;[1 1 1] Attach / Detach
  (Transformation|AttachComponentToComponent (Variables|Default|GetOneHand) (Variables|Character|GetMesh) "Hand_Sword" "KeepRelative" "KeepRelative" "KeepRelative" true))

(event Custom|Detach_OneHand
  ;[1 1 1] Attach / Detach
  (Transformation|AttachComponentToComponent (Variables|Default|GetOneHand) (Variables|Character|GetMesh) "Holster_Sword" "KeepRelative" "KeepRelative" "KeepRelative" true))

(event Input|ActionEvents|InputActionOneHand
  (params (Key :type Key%20Structure :default "None"))
  ;[1 1 1] OneHand Input Key
  (:Pressed
    (switch Utilities|FlowControl|Switch|SwitchonECombatType (Variables|Default|GetCombatType)
      (:NewEnumerator0
        (CallFunction|EquipOneHand))
      (:NewEnumerator1
        (CallFunction|UnequipOneHand)))))

(event EventBeginPlay
  (bind _returnvalue (Game|SpawnActorfromClass "/Game/Weapons/BP_OneHand.BP_OneHand_C" (Math|Transform|MakeTransform "0, 0, 0") "Undefined" self 0))
  (bind _output_get (Variables|Default|SetOneHand _returnvalue))
  (Transformation|AttachComponentToComponent _output_get (Variables|Character|GetMesh) "Holster_Sword" "KeepRelative" "KeepRelative" "KeepRelative" true))

(event Custom|EndAction
  (Variables|Default|SetStateType "NewEnumerator0"))

(event Input|ActionEvents|InputActionAction
  (params (Key :type Key%20Structure :default "None"))
  (:Pressed
    (if (and (Utilities|Enum|Equal(Enum) (Variables|Default|GetCombatType) "NewEnumerator1") (Utilities|Enum|Equal(Enum) (Variables|Default|GetStateType) "NewEnumerator0"))
      (Variables|Default|SetStateType "NewEnumerator3")
      (Animation|PlayAnimMontage "/Game/Character/Animations/OneHand/Sword_Attack_1_Montage.Sword_Attack_1_Montage" 1.0 "None"))))