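; BP_Enemy is an enemy character that spawns a two-handed weapon on its hand socket and reacts to damage.
; Each hit lowers Health, plays a montage, turns it toward the attacker and flashes it red; Health's OnRep updates the widget bar.
; Surviving magic hits trigger a timed effect or a time-dilation slow by throw index, while the melee switch is empty.
; Death ragdolls it away from the attacker, then destroys weapon and actor after a delay.
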(event Custom|EndDead
  (Actor|DestroyActor))

(event EventBeginPlay
  (bind _returnvalue (Game|SpawnActorfromClass "/Game/Weapons/Melee/BP_TwoHand.BP_TwoHand_C" (Math|Transform|MakeTransform "0, 0, 0") "Undefined" self 0))
  (bind _output_get (Variables|Default|SetTwoHand _returnvalue))
  (Transformation|AttachComponentToComponent _output_get (Variables|Character|GetMesh) "Hand_GreatSword" "KeepRelative" "KeepRelative" "KeepRelative" true))

(event Game|Damage|EventAnyDamage
  (params (Damage :type Float%20%28single-precision%29) (DamageType :type Damage%20Type%20Object%20Reference) (InstigatedBy :type Controller%20Object%20Reference) (DamageCauser :type Actor%20Object%20Reference))
  (|SetDaamge Damage InstigatedBy DamageCauser)
  (Animation|PlayAnimMontage "/Game/Character/Animations/Common/HitReaction_Montage.HitReaction_Montage" 3.0 "None")
  (|LookAtAttcker)
  (|HitColor)
  (|CheckDead
    (:NotDead
      (|Hitted))))

(fn ConstructionScript
  (Rendering|Material|SetVectorParameterValueonMaterials (Variables|Character|GetMesh) "BodyColor" (Math|Conversions|ToVector(LinearColor) (Variables|Default|GetBodyColor)))
  (Rendering|Components|TextRender|SetText (Variables|Default|GetTextRender) (Utilities|Text|ToText(String) (Utilities|GetDisplayName self))))

(fn Ragdoll
  (bind _mesh (Variables|Character|GetMesh))
  (Collision|SetCollisionEnabled (Variables|Collision|GetCapsuleComponent) "NoCollision")
  (Physics|SetSimulatePhysics _mesh true)
  (Collision|SetCollisionProfileName _mesh "Ragdoll" true :!class /Script/Engine.PrimitiveComponent)
  (Physics|AddForce _mesh (* (* (Math|Vector|GetUnitDirection(Vector) (Transformation|GetActorLocation (Variables|Default|GetAttacker)) (Transformation|GetActorLocation)) (Variables|Default|GetDamage)) 250000) "None" false))

(fn OnRepHealth
  (bind _aswb_enemy_health (Utilities|Casting|CastToWB_EnemyHealth (UserInterface|GetUserWidgetObject (Variables|Default|GetHealthWidget))))
  (Default|UpdateHelathBar _aswb_enemy_health (Variables|Default|GetHealth) (Math|Float|MakeLiteralFloat 1e+02)))