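; BP_Weapon is a weapon actor that serves as a base, with empty hooks for equipping, unequipping, attacking and ending an action.
; SendDamage damages Characters other than the owner, crediting the owner's instigator controller.
; CanAttack requires the owner's combat type to match the weapon's and its state to be idle.
; It queries and changes owner state through IWeapon and IState interface messages, avoiding casts to the owner's class.
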(event Custom|OnEquipped)

(event Custom|OnUnequipped)

(event EventBeginPlay)

(event Collision|EventActorBeginOverlap
  (params (OtherActor :type Actor%20Object%20Reference)))

(event EventTick
  (params (DeltaSeconds :type Float%20%28single-precision%29)))

(fn ConstructionScript)

(fn SendDamage
  (params (OtherActor :type Actor%20Object%20Reference) (Damage :type Float%20%28single-precision%29))
  (if (!= OtherActor (Components|GetOwner))
    (bind _ascharacter (Utilities|Casting|CastToCharacter OtherActor))
    (Game|Damage|ApplyDamage _ascharacter Damage (Game|GetInstigatorController (Components|GetOwner)) self)
    (return true)
    (else
      (return false))))

(fn Attack)

(fn CanAttack
  (return (and (Utilities|Enum|Equal(Enum) (CallFunction|GetWeaponCombatType) (Variables|Default|GetCombatType)) (CallFunction|IsStateIdling))))

(fn GetWeaponCombatType
  (bind _returnvalue (Components|GetOwner))
  (if (Utilities|DoesObjectImplementInterface _returnvalue "/Game/Interfaces/IWeapon.IWeapon_C")
    (bind _currentcombattype (Class|IWeapon|GetWeaponCombatType(Message) _returnvalue))
    (return _currentcombattype)))

(fn IsStateIdling
  (bind _returnvalue (Components|GetOwner))
  (if (Utilities|DoesObjectImplementInterface _returnvalue "/Game/Interfaces/IState.IState_C")
    (bind _result (Class|IState|IsStateIDling(Message) _returnvalue))
    (return _result)))

(fn SetStateIdling
  (bind _returnvalue (Components|GetOwner))
  (if (Utilities|DoesObjectImplementInterface _returnvalue "/Game/Interfaces/IState.IState_C")
    (Class|IState|SetStateIdling(Message) _returnvalue)))

(fn SetStateAttacking
  (bind _returnvalue (Components|GetOwner))
  (if (Utilities|DoesObjectImplementInterface _returnvalue "/Game/Interfaces/IState.IState_C")
    (Class|IState|SetStateAttacking(Message) _returnvalue)))

(fn SetStateMove
  (params (bMove :type Boolean))
  (bind _returnvalue (Components|GetOwner))
  (if (Utilities|DoesObjectImplementInterface _returnvalue "/Game/Interfaces/IState.IState_C")
    (Class|IState|SetStateMove(Message) _returnvalue bMove)))

(fn SetStateSpelling
  (bind _returnvalue (Components|GetOwner))
  (if (Utilities|DoesObjectImplementInterface _returnvalue "/Game/Interfaces/IState.IState_C")
    (Class|IState|SetStateSpelling(Message) _returnvalue)))

(fn EndAction)