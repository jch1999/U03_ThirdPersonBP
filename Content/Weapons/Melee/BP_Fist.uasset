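; Unarmed fist melee weapon that deals damage through punch and kick hit spheres attached to sockets on the owning character's mesh.
; On BeginPlay it attaches the four limb collisions and disables all sphere components.
; OnCollision enables only the limb matching the attack type, and OffCollision disables them all again.
; Each limb's overlap sends damage taken from the damage component using the current combo count.
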(event OnComponentBeginOverlap(LeftPunch)
  (params (OverlappedComponent :type Primitive%20Component%20Object%20Reference) (OtherActor :type Actor%20Object%20Reference) (OtherComp :type Primitive%20Component%20Object%20Reference) (OtherBodyIndex :type Integer) (bFromSweep :type Boolean) (SweepResult :type Hit%20Result%20Structure%20%28by%20ref%29))
  (CallFunction|SendDamage OtherActor (Default|GetDamage (Variables|Default|GetDamageComopnent) (Variables|Default|GetComboCnt))))

(event OnComponentBeginOverlap(RightPunch)
  (params (OverlappedComponent :type Primitive%20Component%20Object%20Reference) (OtherActor :type Actor%20Object%20Reference) (OtherComp :type Primitive%20Component%20Object%20Reference) (OtherBodyIndex :type Integer) (bFromSweep :type Boolean) (SweepResult :type Hit%20Result%20Structure%20%28by%20ref%29))
  (CallFunction|SendDamage OtherActor (Default|GetDamage (Variables|Default|GetDamageComopnent) (Variables|Default|GetComboCnt))))

(event OnComponentBeginOverlap(LeftKick)
  (params (OverlappedComponent :type Primitive%20Component%20Object%20Reference) (OtherActor :type Actor%20Object%20Reference) (OtherComp :type Primitive%20Component%20Object%20Reference) (OtherBodyIndex :type Integer) (bFromSweep :type Boolean) (SweepResult :type Hit%20Result%20Structure%20%28by%20ref%29))
  (CallFunction|SendDamage OtherActor (Default|GetDamage (Variables|Default|GetDamageComopnent) (Variables|Default|GetComboCnt))))

(event OnComponentBeginOverlap(RightKick)
  (params (OverlappedComponent :type Primitive%20Component%20Object%20Reference) (OtherActor :type Actor%20Object%20Reference) (OtherComp :type Primitive%20Component%20Object%20Reference) (OtherBodyIndex :type Integer) (bFromSweep :type Boolean) (SweepResult :type Hit%20Result%20Structure%20%28by%20ref%29))
  (CallFunction|SendDamage OtherActor (Default|GetDamage (Variables|Default|GetDamageComopnent) (Variables|Default|GetComboCnt))))

(event EventOnCollision
  (params (AttackCollision :type EFistType%20Enum :default "NewEnumerator0"))
  (|CallParentFunction AttackCollision)
  (switch Utilities|FlowControl|Switch|SwitchonEFistType AttackCollision
    (:NewEnumerator1
      (Collision|SetCollisionEnabled (Variables|Default|GetLeftPunch) "QueryAndPhysics"))
    (:NewEnumerator2
      (Collision|SetCollisionEnabled (Variables|Default|GetRightPunch) "QueryAndPhysics"))
    (:NewEnumerator3
      (Collision|SetCollisionEnabled (Variables|Default|GetLeftKick) "QueryAndPhysics"))
    (:NewEnumerator4
      (Collision|SetCollisionEnabled (Variables|Default|GetRightKick) "QueryAndPhysics"))))

(event EventOffCollision
  (|CallParentFunction)
  (CallFunction|SetAllCollisions "NoCollision"))

(event EventBeginPlay
  (|CallParentFunction)
  (Utilities|FlowControl|Sequence
    (:then_0
      (CallFunction|AttachCollisiontoSocket (Variables|Default|GetLeftPunch) "Fist_LeftPunch")
      (CallFunction|AttachCollisiontoSocket (Variables|Default|GetRightPunch) "Fist_RightPunch"))
    (:then_1
      (CallFunction|AttachCollisiontoSocket (Variables|Default|GetLeftKick) "Fist_LeftKick")
      (CallFunction|AttachCollisiontoSocket (Variables|Default|GetRightKick) "Fist_RightKick")
      (CallFunction|SetAllCollisions "NoCollision"))))

(fn ConstructionScript)

(fn AttachCollisiontoSocket
  (params (Collision :type Sphere%20Component%20Object%20Reference) (SocketName :type Name))
  (bind _ascharacter (Utilities|Casting|CastToCharacter (Components|GetOwner)))
  (Transformation|AttachComponentToComponent Collision (Variables|/Script/Engine.Character|GetMesh _ascharacter) SocketName "KeepRelative" "KeepRelative" "KeepRelative" true))

(fn SetAllCollisionsEnabled
  (for _array_element (Actor|GetComponentsByClass "/Script/Engine.SphereComponent")
    (Collision|SetCollisionEnabled _array_element "QueryAndPhysics")))

(fn SetAllCollisionsDisabled
  (for _array_element (Actor|GetComponentsByClass "/Script/Engine.SphereComponent")
    (Collision|SetCollisionEnabled _array_element "NoCollision")))

(fn SetAllCollisions
  (params (CollisionType :type ECollisionEnabled%20Enum :default "NoCollision"))
  (for _array_element (Actor|GetComponentsByClass "/Script/Engine.SphereComponent")
    (Collision|SetCollisionEnabled _array_element CollisionType)))