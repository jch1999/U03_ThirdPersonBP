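; Melee weapon Blueprint that drives a chained combo attack on its owning Character.
; BeginPlay loads every data table row into MeleeDatas, and each entry supplies a montage, play rate, start section and movement permission.
; An Attack during the CanCombo window buffers the next hit, which NextCombo plays by advancing ComboCnt.
; EndAction restores idle and movement and resets the combo, while OnCollision and OffCollision are empty stubs.
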(event Custom|NextCombo
  ;[1 1 1] 콤보 연결 성공 시
  (if (Variables|Default|GetbSucceedCombo)
    (Variables|Default|SetbSucceedCombo false)
    (Math|Integer|IncrementInt (Variables|Default|GetComboCnt)
      (:%20%20
        (CallFunction|PlayComboMontage)))))

(event Custom|EndAction
  ;[1 1 1] 막타 OR 콤보 실패 시
  (CallFunction|SetStateIdling)
  (CallFunction|SetStateMove true)
  (Variables|Default|SetComboCnt 0)
  (Variables|Default|SetbCanCombo false)
  (Variables|Default|SetbSucceedCombo false))

(event EventAttack
  ;[1 1 1] 왼쪽 클릭 시
  (|CallParentFunction)
  (if (Variables|Default|GetbCanCombo)
    (Variables|Default|SetbCanCombo false)
    (Variables|Default|SetbSucceedCombo true)
    (elif (CallFunction|CanAttack)
      (CallFunction|SetStateAttacking)
      (CallFunction|PlayComboMontage))))

(event EventBeginPlay
  ;[1 1 1] Read Data Table
  (|CallParentFunction)
  (bind _outrownames (DataTable|GetDataTableRowNames (Variables|Default|GetDataTable)))
  (for _array_element _outrownames
    (bind _returnvalue (Utilities|GetDataTableRow (Variables|Default|GetDataTable) _array_element)
      (:then
        (Utilities|Array|Add (Variables|Default|GetMeleeDatas) _returnvalue)))))

(fn ConstructionScript
  (|CallParentFunction))

(fn PlayComboMontage
  (bind _meleedatas (Variables|Default|GetMeleeDatas))
  (bind _combocnt (Variables|Default|GetComboCnt))
  (bind _output (Utilities|Array|Get(acopy) _meleedatas _combocnt))
  (bind _ascharacter (Utilities|Casting|CastToCharacter (Components|GetOwner)))
  (Animation|PlayAnimMontage _ascharacter (.animmontage _output) (.playrate _output) (.startsection _output))
  (CallFunction|SetStateMove (.bcanmove _output)))

(fn OnCollision)

(fn OffCollision)