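; BP_Projectile is a magic projectile owned by a BP_Skill_Throw, with a short lifespan set on BeginPlay.
; It reaches its magic and caster through the owner chain.
; SendDamge ignores the caster, spawns an impact emitter at an offset facing from caster to target, passes damage to the magic, then destroys itself.
; Its own overlap event is empty, so nothing here calls SendDamge.
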(event EventBeginPlay
  (Actor|SetLifeSpan 5.0))

(event Collision|EventActorBeginOverlap
  (params (OtherActor :type Actor%20Object%20Reference)))

(event EventTick
  (params (DeltaSeconds :type Float%20%28single-precision%29)))

(fn ConstructionScript)

(fn GetOwnertoSkillThrow
  (bind _asbp_skill_throw (Utilities|Casting|CastToBP_Skill_Throw (Components|GetOwner))
    (:then
      (return _asbp_skill_throw))
    (:CastFailed
      (return 0))))

(fn GetOwnertoMagic
  (return (Default|GetOwnertoMagic (CallFunction|GetOwnertoSkillThrow))))

(fn SendDamge
  (params (OtherActor :type Actor%20Object%20Reference) (Damage :type Float%20%28single-precision%29) (ImpatPaticle :type Particle%20System%20Object%20Reference) (ImpactLocation :type Vector) (ImpactScale :type Vector :default "1.000000,1.000000,1.000000"))
  (bind _asbp_magic (CallFunction|GetOwnertoMagic))
  (bind _returnvalue (Components|GetOwner _asbp_magic))
  (if (!= OtherActor _returnvalue)
    (Effects|SpawnEmitteratLocation ImpatPaticle (+ ImpactLocation (Transformation|GetActorLocation)) (Math|Rotator|FindLookatRotation (Transformation|GetActorLocation _returnvalue) (Transformation|GetActorLocation OtherActor)) ImpactScale)
    (Default|SendDamage (CallFunction|GetOwnertoMagic) OtherActor Damage)
    (Actor|DestroyActor)))