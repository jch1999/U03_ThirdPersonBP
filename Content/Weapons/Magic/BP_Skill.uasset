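; BP_Skill is a skill actor owned by a BP_Magic weapon, with empty Spell, OnSet and OnUnset events that appear to be hooks for child skills.
; Spelled returns the owning magic to its idling state and calls SetStateMove with true.
; Helper functions cast up the owner chain from the skill to its BP_Magic, then to that magic's owning Character.
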(event Custom|Spell)

(event Custom|Spelled
  (bind _asbp_magic (CallFunction|GetOwnertoMagic))
  (Default|SetStateIdling _asbp_magic)
  (Default|SetStateMove _asbp_magic true))

(event Custom|OnSet)

(event Custom|OnUnset)

(fn ConstructionScript)

(fn GetOwnertoMagic
  (bind _asbp_magic (Utilities|Casting|CastToBP_Magic (Components|GetOwner)))
  (return _asbp_magic))

(fn GetOwnertoCharacter
  (bind _ascharacter (Utilities|Casting|CastToCharacter (Components|GetOwner (CallFunction|GetOwnertoMagic))))
  (return _ascharacter))