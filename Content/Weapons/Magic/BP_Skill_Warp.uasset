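; Warp magic skill that moves its owner to the point under the cursor on world-static geometry.
; While equipped, a decal previews that point, aligned to the surface normal and hidden without a hit.
; Spell stores the hit location, locks movement and plays a montage, or ends the action without a hit; Spelled restores movement.
; DoWarp, not called within this Blueprint, performs a swept move raised by capsule half-height.
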(event Custom|DoWarp
  (bind _warplocation (Variables|Default|GetWarpLocation))
  (if (Variables|Default|GetbCanWarp)
    (Transformation|SetActorLocation (CallFunction|GetOwnertoCharacter) (Math|Vector|MakeVector (.x _warplocation) (.y _warplocation) (+ (.z _warplocation) (Components|Capsule|GetScaledCapsuleHalfHeight (Variables|/Script/Engine.Character|GetCapsuleComponent (CallFunction|GetOwnertoCharacter))))) true false)
    (Variables|Default|SetbCanWarp false)))

(event EventOnSet
  (|CallParentFunction)
  (Variables|Default|SetbEquipped true))

(event EventOnUnset
  (|CallParentFunction)
  (Variables|Default|SetbEquipped false))

(event EventTick
  (params (DeltaSeconds :type Float%20%28single-precision%29))
  (if (Variables|Default|GetbEquipped)
    (bind (_location _impactnormal) (Utilities|GetCursorInfo)
      (:True
        (Transformation|SetWorldLocation (Variables|Default|GetDecal) _location false false)
        (Transformation|SetWorldRotation (Variables|Default|GetDecal) (Math|Conversions|RotationFromXVector _impactnormal) false false)
        (Rendering|SetVisibility (Variables|Default|GetDecal) true false))
      (:False
        (Rendering|SetVisibility (Variables|Default|GetDecal) false false :!label _label)))
    (else
      (goto _label))))

(event EventSpell
  (|CallParentFunction)
  (bind _location (Utilities|GetCursorInfo)
    (:True
      (Variables|Default|SetWarpLocation _location)
      (Variables|Default|SetbCanWarp true)
      (Default|SetStateMove (CallFunction|GetOwnertoMagic) false)
      (Animation|PlayAnimMontage (CallFunction|GetOwnertoCharacter) "/Game/Character/Animations/Magic/MG_InstantHeal_Montage.MG_InstantHeal_Montage" 1.5 "None"))
    (:False
      (Variables|Default|SetbCanWarp false)
      (Default|EndAction (CallFunction|GetOwnertoMagic)))))

(event EventSpelled
  (|CallParentFunction)
  (Default|SetStateMove (CallFunction|GetOwnertoMagic) true))

(event EventBeginPlay
  (|CallParentFunction)
  (Rendering|SetVisibility (Variables|Default|GetDecal) false false))

(fn ConstructionScript
  (|CallParentFunction))